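; Player controller that handles targeting and interacting with items, menu opening, and inspection rotation input.
; Each tick a camera-forward line trace finds a BP_BaseItem, firing hover and unhover on changes and updating the UI; a miss clears the target, while non-item hits keep it.
; Interact calls OnInteract on the current target, and left mouse toggles rotation during inspection.
; ToggleInputMode switches between UI-only input with cursor and game-only input.
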(event `self.ReceiveTick`
  (params (DeltaSeconds :type "Float (single-precision)"))
  (bind _returnvalue (`GameplayStatics.GetPlayerCameraManager` 0))
  (bind _returnvalue_2 (`PlayerCameraManager.GetCameraLocation` _returnvalue))
  (bind (_outhit _returnvalue_3) (`KismetSystemLibrary.LineTraceSingle` _returnvalue_2 (+ _returnvalue_2 (* (`self.GetActorForwardVector` _returnvalue) (`self.LineTraceLength`))) "TraceTypeQuery3"))
  (if _returnvalue_3
    (bind _asbp_base_item (cast `/Game/Blueprints/Items/BP_BaseItem` (`.HitActor` (`GameplayStatics.BreakHitResult` _outhit))))
    (`self.SetCurrentTarget` _asbp_base_item)
    (else
      (`self.SetCurrentTarget` null))))

(event `InputAction|Interact`
  (params (Key :type "Key Structure"))
  (:`Pressed`
    (bind _currenttarget (`self.CurrentTarget`)
      (:`then`
        (`/Game/Blueprints/Items/BP_BaseItem.On Interact` _currenttarget))
      (:`else`))))

(event `InputAction|OpenMenu`
  (params (Key :type "Key Structure"))
  ;[1 1 1] UI
  (:`Pressed`
    (`/Game/Blueprints/Widgets/WB_Main.OpenMenu` (`/Game/Blueprints/BP_BlueprintLibrary.GetVincentsUI`))))

(event `Toggle Input Mode`
  (params (InputToUI :type Boolean))
  ;[1 1 1] UI
  (if InputToUI
    (set `self.bShowMouseCursor` true)
    (`WidgetBlueprintLibrary.SetInputMode_UIOnlyEx` self null)
    (else
      (set `self.bShowMouseCursor` false)
      (`WidgetBlueprintLibrary.SetInputMode_GameOnly` self))))

(event `Key|LeftMouseButton`
  (params (Key :type "Key Structure"))
  (bind _character (`/Game/Blueprints/BP_BlueprintLibrary.GetVincentsCharacter`))
  (:`Pressed`
    (if (`/Game/Blueprints/BP_VincentsCharacter.In Inspection` _character)
      (set `/Game/Blueprints/BP_VincentsCharacter.In Inspection Rotation` true _character)))
  (:`Released`
    (set `/Game/Blueprints/BP_VincentsCharacter.In Inspection Rotation` false _character)))

(fn `SetCurrentTarget`
  (params (NewTarget :type "/Game/Blueprints/Items/BP_BaseItem Object Reference"))
  (if (!= (`self.CurrentTarget`) NewTarget)
    (`|ExecutionSequence`
      (:`then_0`
        (bind _currenttarget (`self.CurrentTarget`)
          (:`then`
            (`/Game/Blueprints/Items/BP_BaseItem.On Unhover` _currenttarget))
          (:`else`)))
      (:`then_1`
        (`/Engine/EditorBlueprintResources/StandardMacros.IsValid` NewTarget
          (:`Is Valid`
            (`/Game/Blueprints/Items/BP_BaseItem.On Hover` NewTarget))))
      (:`then_2`
        (`/Game/Blueprints/Widgets/WB_Main.SetCurrentTarget` (`/Game/Blueprints/BP_BlueprintLibrary.GetVincentsUI`) NewTarget)
        (set `self.CurrentTarget` NewTarget)))))

(fn `UserConstructionScript`)