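; BP_Level_Father is a level-module actor that tracks paintings and completes the level once enough are registered.
; OnPaintingAdded and OnPaintingRemoved maintain the Paintings array, and an addition that brings its length to at least PaintingsCount triggers End Level.
; End Level calls OnLevelComplete on every painting in the array, then on the Father reference.
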(event `On Painting Added`
  (params (Painting :type "/Game/Blueprints/Items/BP_PaintingSlot Object Reference"))
  (bind _paintings (`self.Paintings`))
  (`KismetArrayLibrary.Array_Add` _paintings Painting)
  (if (>= (`KismetArrayLibrary.Array_Length` _paintings) (`self.PaintingsCount`))
    (for _array_element (`self.Paintings`)
      (`/Game/Blueprints/Items/BP_PaintingSlot.On Level Complete` _array_element))
    (`/Game/Blueprints/Items/BP_ItemFather.OnLevelComplete` (`self.Father`))))

(event `On Painting Removed`
  (params (Painting :type "/Game/Blueprints/Items/BP_PaintingSlot Object Reference"))
  (`KismetArrayLibrary.Array_RemoveItem` (`self.Paintings`) Painting))

(fn `UserConstructionScript`
  (`parent.UserConstructionScript`))