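; BP_LevelManager tracks progress through an ordered array of levels and advances from one to the next.
; On BeginPlay it registers itself with Vincent's game mode.
; When a level completes, it calls that level's OnComplete and uses the returned value as a delay before advancing.
; It then increments the index and calls OnEnter on the next level, if one remains.
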(event `self.ReceiveBeginPlay`
  (set `/Game/Blueprints/BP_GameMode.LevelManager` self (`/Game/Blueprints/BP_BlueprintLibrary.GetVincentsGameMode`)))

(event `On Level Complete`
  (bind _duration (`/Game/Blueprints/LevelModule/BP_Level.OnComplete` (`self.GetCurrentLevel`)))
  (`KismetSystemLibrary.Delay` _duration)
  (`self.EnterNextLevel`))

(fn `EnterNextLevel`
  (bind _level_index (`self.Level Index`))
  (`/Engine/EditorBlueprintResources/StandardMacros.IncrementInt` _level_index
    (:`  `
      (if (< _level_index (`KismetArrayLibrary.Array_Length` (`self.Levels`)))
        (`/Game/Blueprints/LevelModule/BP_Level.OnEnter` (`|GetArrayItem` (`self.Levels`) (`self.Level Index`)))))))

(fn `GetCurrentLevel`
  (returns (Output :type "/Game/Blueprints/LevelModule/BP_Level Object Reference"))
  (return (`|GetArrayItem` (`self.Levels`) (`self.Level Index`))))

(fn `UserConstructionScript`)