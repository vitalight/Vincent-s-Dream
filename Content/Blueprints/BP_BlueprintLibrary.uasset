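; Blueprint function library giving shortcut access to the game's core Vincents objects and item data.
; Getters cast the game mode, player 0's pawn and controller, and read the main UI, level manager and sound actor from the game mode.
; GetItemInfo looks up Table_Item using the item type enum's string as row name, printing an error if missing.
; One enum value bypasses the table and returns a hardcoded test item.
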(fn `GetItemInfo`
  (params (Type :type "/Game/Blueprints/ItemModule/EItemType Enum" :default "NewEnumerator3"))
  (returns (ItemTableRow :type "/Game/Blueprints/ItemModule/SItemTableRow Structure"))
  (bind _returnvalue (`KismetStringLibrary.Conv_StringToName` (`|GetEnumeratorNameAsString` Type)))
  (if (`|EnumInequality` Type "NewEnumerator4")
    (bind _returnvalue_2 (`|GetDataTableRow` "/Game/Blueprints/ItemModule/Table_Item.Table_Item" _returnvalue)
      (:`then`
        (return _returnvalue_2))
      (:`RowNotFound`
        (`KismetSystemLibrary.PrintString` null (`KismetStringLibrary.Concat_StrStr` "Error: Invalid item type " (`KismetStringLibrary.Conv_NameToString` _returnvalue)))
        (return)))
    (else
      (return (make `/Game/Blueprints/ItemModule/SItemTableRow` "测试道具" "这是一个测试道具")))))

(fn `GetVincentsCharacter`
  (returns (Character :type "/Game/Blueprints/BP_VincentsCharacter Object Reference"))
  (bind _asbp_vincents_character (cast `/Game/Blueprints/BP_VincentsCharacter` (`GameplayStatics.GetPlayerPawn` null))
    (:`then`
      (return _asbp_vincents_character))
    (:`CastFailed`
      (return null))))

(fn `GetVincentsGameMode`
  (returns (GameMode :type "/Game/Blueprints/BP_GameMode Object Reference"))
  (bind _asbp_game_mode (cast `/Game/Blueprints/BP_GameMode` (`GameplayStatics.GetGameMode` null))
    (:`then`
      (return _asbp_game_mode))
    (:`CastFailed`
      (return null))))

(fn `GetVincentsLevelManager`
  (returns (LevelManager :type "/Game/Blueprints/LevelModule/BP_LevelManager Object Reference"))
  (return (`/Game/Blueprints/BP_GameMode.LevelManager` (`self.GetVincentsGameMode` null))))

(fn `GetVincentsPlayerController`
  (returns (`Player Controller` :type "/Game/Blueprints/BP_PlayerController Object Reference"))
  (bind _asbp_player_controller (cast `/Game/Blueprints/BP_PlayerController` (`GameplayStatics.GetPlayerController` null))
    (:`then`
      (return _asbp_player_controller))
    (:`CastFailed`
      (return null))))

(fn `GetVincentsSoundActor`
  (returns (SoundActor :type "/Game/Blueprints/Sounds/BP_SoundActor Object Reference"))
  (return (`/Game/Blueprints/BP_GameMode.SoundActor` (`self.GetVincentsGameMode` null))))

(fn `GetVincentsUI`
  (returns (UI :type "/Game/Blueprints/Widgets/WB_Main Object Reference"))
  (return (`/Game/Blueprints/BP_GameMode.Main UI` (`self.GetVincentsGameMode` null))))