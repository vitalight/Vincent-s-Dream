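; Backpack component that holds an inventory of items and tracks which one is selected.
; Items live in a map keyed by item type, with AddItem creating an entry or incrementing the found entry's amount.
; Selection indexes into the map's values, stepping up or down with modulo wraparound and skipping empty inventories.
; Event dispatchers announce item and selection changes, and getters expose all items or the selected one.
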(fn `AddItem`
  (params (ItemType :type "/Game/Blueprints/ItemModule/EItemType Enum" :default "NewEnumerator3"))
  (bind (_value _returnvalue) (`BlueprintMapLibrary.Map_Find` (`self.Items`) ItemType))
  (`|ExecutionSequence`
    (:`then_0`
      (if _returnvalue
        (setmembers `/Game/Blueprints/ItemModule/SBackpackItem` :`StructRef` _value :`Amount` (+ (`.Amount_5_59F380E7462341A901E13997ABF3982E` (break `/Game/Blueprints/ItemModule/SBackpackItem` _value)) 1))
        (else
          (`BlueprintMapLibrary.Map_Add` (`self.Items`) ItemType (make `/Game/Blueprints/ItemModule/SBackpackItem` ItemType 1)))))
    (:`then_1`
      (`self.OnItemsUpdate`))))

(fn `GetAllItems`
  (returns (Values :type "Array of /Game/Blueprints/ItemModule/SBackpackItem Structure"))
  (bind _values (`BlueprintMapLibrary.Map_Values` (`self.Items`)))
  (return _values))

(fn `GetSelectedItem`
  (returns (Output :type "/Game/Blueprints/ItemModule/SBackpackItem Structure (by ref)"))
  (bind _values (`BlueprintMapLibrary.Map_Values` (`self.Items`)))
  (return (`|GetArrayItem` _values (`self.SelectedIndex`))))

(fn `UpdateSelectedIndex`
  (params (Increase :type Boolean))
  (bind _selectedindex (`self.SelectedIndex`))
  (bind _returnvalue (`BlueprintMapLibrary.Map_Length` (`self.Items`)))
  (if (!= _returnvalue 0)
    (`|ExecutionSequence`
      (:`then_0`
        (if Increase
          (`/Engine/EditorBlueprintResources/StandardMacros.IncrementInt` _selectedindex)
          (else
            (`/Engine/EditorBlueprintResources/StandardMacros.DecrementInt` _selectedindex))))
      (:`then_1`
        (set `self.SelectedIndex` (mod (+ (`self.SelectedIndex`) _returnvalue) _returnvalue))
        (`self.OnSelectedIndexUpdate`)))))