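; BP_SoundActor is the game's music player, registering itself with Vincent's game mode on BeginPlay so other code can reach it.
; PlayMusic maps a music type to a track stored in NextSound, then fades out its single AudioComponent, waits, swaps the sound and fades back in.
; The fades run in sequence rather than as a crossfade, and an invalid track leaves the music silent.
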(event `self.ReceiveBeginPlay`
  (set `/Game/Blueprints/BP_GameMode.SoundActor` self (`/Game/Blueprints/BP_BlueprintLibrary.GetVincentsGameMode`)))

(event `Play Music`
  (params (Type :type "/Game/Blueprints/Sounds/ESoundType Enum" :default "NewEnumerator0"))
  (bind _fadeduration (`self.FadeDuration`))
  (bind _audiocomponent (`self.AudioComponent`))
  (bind _nextsound (`self.NextSound`))
  (`|ExecutionSequence`
    (:`then_0`
      (set `self.NextSound` (select `/Game/Blueprints/Sounds/ESoundType` Type :`NewEnumerator0` "/Game/Arts/Audio/Bgm_Main.Bgm_Main" :`NewEnumerator3` "/Game/Arts/Audio/DrawingAppear.DrawingAppear" :`NewEnumerator1` "/Game/Arts/Audio/Bgm_Japan_01.Bgm_Japan_01" :`NewEnumerator2` "/Game/Arts/Audio/Bgm_Japan_02.Bgm_Japan_02" :!type "SoundWave Object Reference")))
    (:`then_1`
      (`AudioComponent.FadeOut` _audiocomponent _fadeduration 0.0)
      (`KismetSystemLibrary.Delay` _fadeduration)
      (`AudioComponent.SetSound` _audiocomponent _nextsound)
      (`/Engine/EditorBlueprintResources/StandardMacros.IsValid` _nextsound
        (:`Is Valid`
          (`AudioComponent.FadeIn` _audiocomponent _fadeduration 1.0 0.0))))))

(fn `UserConstructionScript`)