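; BP_ItemDrawer is an interactable drawer that slides open and closed.
; The construction script caches the actor's location and derives an open target from DrawDistance rotated by the actor's rotation.
; OnInteract plays the OpenDrawer sound, then a FlipFlop alternately plays and reverses a timeline that lerps the whole actor between those positions without sweep.
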(event `self.On Interact`
  (`GameplayStatics.PlaySoundAtLocation` "/Game/Arts/Audio/OpenDrawer.OpenDrawer" (`self.K2_GetActorLocation`) (struct) 1.0 1.0 0.0 null null null)
  (`/Engine/EditorBlueprintResources/StandardMacros.FlipFlop`
    (:`A`
      (bind (_direction _move_item) (`Timeline|Timeline_0` :!label _label)
        (:`Update`
          (`self.K2_SetActorLocation` (`KismetMathLibrary.VLerp` (`self.DefaultLocation`) (`self.DrawTarget`) _move_item)))))
    (:`B`
      (goto _label :!via `Reverse`))))

(fn `UserConstructionScript`
  (`parent.UserConstructionScript`)
  (bind _output_get (set `self.DefaultLocation` (`self.K2_GetActorLocation`)))
  (set `self.DrawTarget` (+ _output_get (`KismetMathLibrary.GreaterGreater_VectorRotator` (`self.DrawDistance`) (`self.K2_GetActorRotation`)))))