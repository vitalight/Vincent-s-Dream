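; BP_BaseItem is a base item that highlights on hover and responds to interaction.
; OnInteract adds a collectable item to the Vincent player controller's Backpack and destroys the actor; otherwise a FlipFlop toggles the mesh between two scales.
; OnHover enables custom depth on the mesh unless Vincent's character is in inspection, and OnUnhover disables it.
; Click and cursor-over events are empty, with disconnected debug prints left behind.
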(event `self.ReceiveActorOnClicked`
  (params (ButtonPressed :type "Key Structure")))

(event `self.Box.OnClicked`
  (params (TouchedComponent :type "PrimitiveComponent Object Reference") (ButtonPressed :type "Key Structure")))

(event `self.Box.OnBeginCursorOver`
  (params (TouchedComponent :type "PrimitiveComponent Object Reference")))

(event `On Interact`
  (bind _isa (`/Engine/EditorBlueprintResources/StandardMacros.FlipFlop`)
    (:`A`
      _)
    (:`B`
      _))
  (if (`self.CanBeCollected`)
    (`/Game/Blueprints/ItemModule/BP_BackpackComponent.AddItem` (`/Game/Blueprints/BP_PlayerController.Backpack` (`/Game/Blueprints/BP_BlueprintLibrary.GetVincentsPlayerController`)) self)
    (`self.K2_DestroyActor` self)
    (else
      (`SceneComponent.SetRelativeScale3D` (`self.StaticMesh`) (select `bool` _isa :`false` (0.2 0.2 0.2) :`true` (0.3 0.3 0.3) :!type "Vector Structure")))))

(event `On Hover`
  (`PrimitiveComponent.SetRenderCustomDepth` (`self.StaticMesh`) (not (`/Game/Blueprints/BP_VincentsCharacter.In Inspection` (`/Game/Blueprints/BP_BlueprintLibrary.GetVincentsCharacter`)))))

(event `On Unhover`
  (`PrimitiveComponent.SetRenderCustomDepth` (`self.StaticMesh`) false))

(fn `UserConstructionScript`)