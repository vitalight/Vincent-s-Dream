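; BP_PaintingSlot is an interactable frame slot where the player places and retrieves paintings from the backpack.
; Interacting with an occupied slot returns its painting to the backpack and shows the empty mount.
; An empty slot accepts a selected painting item, copying its material, scale and type onto its mesh with a sound.
; It notifies the current BP_Level_Father when paintings of the Painting type are added or removed.
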(event `self.On Interact`
  (bind _staticmesh (`self.StaticMesh`))
  (bind _backpack (`/Game/Blueprints/BP_PlayerController.Backpack` (`/Game/Blueprints/BP_BlueprintLibrary.GetVincentsPlayerController`)))
  (bind _backpack_2 (`/Game/Blueprints/BP_PlayerController.Backpack` (`/Game/Blueprints/BP_BlueprintLibrary.GetVincentsPlayerController`)))
  (bind (_output _valid) (`/Game/Blueprints/ItemModule/BP_BackpackComponent.GetSelectedItem` _backpack_2))
  (if _valid
    (bind _valid_2 (`self.TakePainting` _backpack_2))
    (if (not _valid_2)
      (bind (_itemtype _amount _itemreference) (break `/Game/Blueprints/ItemModule/SBackpackItem` _output))
      (switch `/Game/Blueprints/ItemModule/EItemType` _itemtype
        (:`NewEnumerator7`
          _)
        (:`NewEnumerator8`
          _)
        (:`NewEnumerator9`
          _)
        (:`NewEnumerator10`
          _)
        (:`NewEnumerator11`
          _)
        (:`NewEnumerator12`
          _))
      (`self.TakePainting` _backpack)
      (`/Game/Blueprints/ItemModule/BP_BackpackComponent.RemoveItem` _backpack _itemtype)
      (bind _output_get (set `self.PaintingReference` _itemreference))
      (`GameplayStatics.PlaySoundAtLocation` "/Game/Arts/Audio/DrawingInFrame.DrawingInFrame" (`self.K2_GetActorLocation`) (struct) 1.0 1.0 0.0 null null null)
      (bind _staticmesh_2 (`/Game/Blueprints/Items/BP_BaseItem.StaticMesh` _output_get))
      (`PrimitiveComponent.SetMaterial` _staticmesh 0 (`PrimitiveComponent.GetMaterial` _staticmesh_2 0))
      (`SceneComponent.SetWorldScale3D` _staticmesh (`SceneComponent.K2_GetComponentScale` _staticmesh_2))
      (`SceneComponent.SetVisibility` (`self.StaticMesh`) true false)
      (`SceneComponent.SetVisibility` (`self.Mount`) false false)
      (set `self.Type` (`/Game/Blueprints/Items/BP_BaseItem.Type` _output_get))
      (bind _asbp_level_father (cast `/Game/Blueprints/LevelModule/BP_Level_Father` (`/Game/Blueprints/LevelModule/BP_LevelManager.GetCurrentLevel` (`/Game/Blueprints/BP_BlueprintLibrary.GetVincentsLevelManager`))))
      (if (`|EnumEquality` _itemtype (`self.Painting`))
        (`/Game/Blueprints/LevelModule/BP_Level_Father.On Painting Added` _asbp_level_father self)))
    (else
      (bind _valid_3 (`self.TakePainting` _backpack_2))
      (if _valid_3
        _))))

(fn `TakePainting`
  (params (Backpack :type "/Game/Blueprints/ItemModule/BP_BackpackComponent Object Reference"))
  (returns (Valid :type Boolean))
  (bind _paintingreference (`self.PaintingReference`))
  (`/Engine/EditorBlueprintResources/StandardMacros.IsValid` _paintingreference
    (:`Is Valid`
      (`/Game/Blueprints/ItemModule/BP_BackpackComponent.AddItem` Backpack _paintingreference)
      (`SceneComponent.SetVisibility` (`self.StaticMesh`) false false)
      (`SceneComponent.SetVisibility` (`self.Mount`) true false)
      (if (`|EnumEquality` (`/Game/Blueprints/Items/BP_BaseItem.Type` _paintingreference) (`self.Painting`))
        (bind _asbp_level_father (cast `/Game/Blueprints/LevelModule/BP_Level_Father` (`/Game/Blueprints/LevelModule/BP_LevelManager.GetCurrentLevel` (`/Game/Blueprints/BP_BlueprintLibrary.GetVincentsLevelManager`))))
        (`/Game/Blueprints/LevelModule/BP_Level_Father.On Painting Removed` _asbp_level_father self))
      (set `self.PaintingReference` null)
      (set `self.Type` "NewEnumerator15")
      (return true))
    (:`Is Not Valid`
      (return false))))

(fn `UserConstructionScript`
  (`parent.UserConstructionScript`))