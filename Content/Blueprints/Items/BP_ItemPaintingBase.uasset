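; Base Blueprint for an interactable painting item with a text widget that fades at level end.
; BeginPlay writes its TipText into the WB_PaintingText widget, and interaction plays a paper sound at its location.
; On level end, it copies the Front and Back textures into a dynamic M_TwoSided_Fade material, whose Opacity the Fade timeline drives.
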(event `self.ReceiveBeginPlay`
  (`parent.ReceiveBeginPlay`)
  (bind _aswb_painting_text (cast `/Game/Blueprints/Widgets/WB_PaintingText` (`WidgetComponent.GetUserWidgetObject` (`self.Text`))))
  (`TextBlock.SetText` (`/Game/Blueprints/Widgets/WB_PaintingText.Txt` _aswb_painting_text) (`self.TipText`)))

(event `self.On Interact`
  (`parent.On Interact`)
  (`GameplayStatics.PlaySoundAtLocation` "/Game/Arts/Audio/Paper.Paper" (`self.K2_GetActorLocation`) (struct) 1.0 1.0 0.0 null null null))

(event `On Level End`
  (bind _asmaterial_instance_constant (cast `MaterialInstanceConstant` (`PrimitiveComponent.GetMaterial` (`self.StaticMesh`) 0)))
  (bind _returnvalue (`MaterialInstanceConstant.K2_GetTextureParameterValue` _asmaterial_instance_constant "Front"))
  (bind _returnvalue_2 (`MaterialInstanceConstant.K2_GetTextureParameterValue` _asmaterial_instance_constant "Back"))
  (bind _returnvalue_3 (`PrimitiveComponent.CreateDynamicMaterialInstance` (`self.StaticMesh`) 0 "/Game/Arts/Materials/M_TwoSided_Fade.M_TwoSided_Fade" "None"))
  (`MaterialInstanceDynamic.SetTextureParameterValue` _returnvalue_3 "Front" _returnvalue)
  (`MaterialInstanceDynamic.SetTextureParameterValue` _returnvalue_3 "Back" _returnvalue_2)
  (bind (_direction _move_item) (`Timeline|Fade` :!via `PlayFromStart`)
    (:`Update`
      (`MaterialInstanceDynamic.SetScalarParameterValue` _returnvalue_3 "Opacity" _move_item))))

(fn `UserConstructionScript`
  (`parent.UserConstructionScript`))