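; Inspectable item that the player brings in front of the first-person camera, rotates, and optionally collects into the backpack.
; A timeline lerps it to a camera-relative pose (backpack items snap there) while its trace channel is ignored.
; Yaw and pitch turn it around camera axes when allowed.
; Ending inspection either reverses the timeline or hides the item, adding it to the backpack if not already there.
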(event `self.On Interact`
  (`/Game/Blueprints/BP_VincentsCharacter.On Inspection` (`/Game/Blueprints/BP_BlueprintLibrary.GetVincentsCharacter`)))

(event `On Inspection`
  (`PrimitiveComponent.SetCollisionResponseToChannel` (`self.StaticMesh`) "ECC_GameTraceChannel1" "ECR_Ignore")
  (bind _output_get (set `self.ItemLocation` (`self.K2_GetActorLocation`)))
  (bind _inspectlocationworld (`self.GetWorldInspectLocation`))
  (bind _output_get_2 (set `self.ItemRotation` (`self.K2_GetActorRotation`)))
  (bind _default_inspect_rotation (`self.GetWorldDefaultInspectRotation`))
  (if (`self.InBackPack`)
    (`self.K2_SetActorLocationAndRotation` _inspectlocationworld _default_inspect_rotation)
    (else
      (bind (_direction _move_item) (`Timeline|Timeline_0` :!label _label)
        (:`Update`
          (`self.K2_SetActorLocationAndRotation` (`KismetMathLibrary.VLerp` _output_get _inspectlocationworld _move_item) (`KismetMathLibrary.RLerp` _output_get_2 _default_inspect_rotation _move_item)))
        (:`Finished`
          (if (not (`/Game/Blueprints/BP_VincentsCharacter.In Inspection` (`/Game/Blueprints/BP_BlueprintLibrary.GetVincentsCharacter`)))
            (`PrimitiveComponent.SetCollisionResponseToChannel` (`self.StaticMesh`) "ECC_GameTraceChannel1" "ECR_Block")))))))

(event `On End Inspection`
  (if (`self.CollectAfterInspection`)
    (`PrimitiveComponent.SetCollisionResponseToChannel` (`self.StaticMesh`) "ECC_GameTraceChannel1" "ECR_Block")
    (if (not (`self.InBackPack`))
      (`/Game/Blueprints/ItemModule/BP_BackpackComponent.AddItem` (`/Game/Blueprints/BP_PlayerController.Backpack` (`/Game/Blueprints/BP_BlueprintLibrary.GetVincentsPlayerController`)) (`self.Type`)))
    (`self.SetActorHiddenInGame` true)
    (`self.K2_SetActorLocation` (0.0 0.0 0.0))
    (goto _label :!via `SetNewTime`)
    (else
      (goto _label :!via `Reverse`))))

(fn `Add Pitch`
  (params (Pitch :type "Float (double-precision)"))
  (if (`self.PitchRotatable`)
    (`self.K2_AddActorWorldRotation` (`KismetMathLibrary.RotatorFromAxisAndAngle` (`SceneComponent.GetRightVector` (`/Game/Blueprints/BP_VincentsCharacter.FirstPersonCamera` (`/Game/Blueprints/BP_BlueprintLibrary.GetVincentsCharacter`))) (* Pitch -1.0)))))

(fn `Add Yaw`
  (params (Yaw :type "Float (double-precision)"))
  (if (`self.YawRotatable`)
    (`self.K2_AddActorWorldRotation` (`KismetMathLibrary.RotatorFromAxisAndAngle` (`SceneComponent.GetUpVector` (`/Game/Blueprints/BP_VincentsCharacter.FirstPersonCamera` (`/Game/Blueprints/BP_BlueprintLibrary.GetVincentsCharacter`))) (* Yaw -1.0)))))

(fn `GetWorldDefaultInspectRotation`
  (returns (`Default Inspect Rotation` :type "Rotator Structure"))
  (bind _firstpersoncamera (`/Game/Blueprints/BP_VincentsCharacter.FirstPersonCamera` (`/Game/Blueprints/BP_BlueprintLibrary.GetVincentsCharacter`)))
  (return (`KismetMathLibrary.ComposeRotators` (`SceneComponent.K2_GetComponentRotation` _firstpersoncamera) (`KismetMathLibrary.ComposeRotators` (`KismetMathLibrary.ComposeRotators` (`KismetMathLibrary.RotatorFromAxisAndAngle` (`SceneComponent.GetForwardVector` _firstpersoncamera) (.roll (`self.DefaultInspectRotation`))) (`KismetMathLibrary.RotatorFromAxisAndAngle` (`SceneComponent.GetRightVector` _firstpersoncamera) (.pitch (`self.DefaultInspectRotation`)))) (`KismetMathLibrary.RotatorFromAxisAndAngle` (`SceneComponent.GetUpVector` _firstpersoncamera) (.yaw (`self.DefaultInspectRotation`)))))))

(fn `GetWorldInspectLocation`
  (returns (InspectLocationWorld :type "Vector Structure"))
  (bind _firstpersoncamera (`/Game/Blueprints/BP_VincentsCharacter.FirstPersonCamera` (`/Game/Blueprints/BP_BlueprintLibrary.GetVincentsCharacter`)))
  (return (+ (`KismetMathLibrary.GreaterGreater_VectorRotator` (`self.InspectLocation`) (`SceneComponent.K2_GetComponentRotation` _firstpersoncamera)) (`SceneComponent.K2_GetComponentLocation` _firstpersoncamera))))

(fn `UserConstructionScript`
  (`parent.UserConstructionScript`))